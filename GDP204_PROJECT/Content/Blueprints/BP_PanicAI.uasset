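; BP_PanicAI is an AI pawn that approaches the player on sight, then flees in a panic.
; PawnSensing sets a seeing flag and starts an AI MoveTo toward the player character.
; Reaching the player triggers RunAway, which moves to a random reachable point around the pawn.
; Each successful flee move clears the flag and calls RunAway again, forming an endless wander loop.
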(event OnSeePawn(PawnSensing)
  (params (Pawn :type Pawn%20Object%20Reference))
  ;[1 1 1] When the AI can see the player, chase them
  (Variables|Default|SetisSeeingPlayer true)
  (CallFunction|FollowPlayer))

(event Custom|FollowPlayer
  ;[1 1 1] When seeing is true, got to player location, then run away
  (if (Variables|Default|GetisSeeingPlayer)
    (AI|AIMoveTo self "0, 0, 0" (Game|GetPlayerCharacter 0) 5.0 false
      (:OnSuccess
        (CallFunction|RunAway)))))

(event Custom|RunAway
  ;[1 1 1] Got to a random location, then a new random location and loop
  (AI|AIMoveTo self (.RandomLocation (AI|Navigation|GetRandomReachablePointinRadius (Transformation|GetActorLocation) 1.5e+03 0 0)) 0 5.0 false
    (:OnSuccess
      (Variables|Default|SetisSeeingPlayer false)
      (CallFunction|RunAway))))

(event EventBeginPlay)

(event Collision|EventActorBeginOverlap
  (params (OtherActor :type Actor%20Object%20Reference)))

(event EventTick
  (params (DeltaSeconds :type Float%20%28single-precision%29)))

(fn ConstructionScript)